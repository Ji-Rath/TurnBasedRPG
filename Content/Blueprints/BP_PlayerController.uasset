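; Player controller for turn-based battle scenes that takes control of characters as their turns come up.
; On BeginPlay it adds inventory and dialogue widgets to the screen and binds to the BP_BattleSceneGameMode turn event.
; HandleTurn possesses the current turn's pawn if it is not already controlled and has no valid controller, then creates a new battle UI widget.
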(event EventBeginPlay
  (bind _returnvalue (UserInterface|CreateWidget "/Game/Blueprints/Widgets/Widget_Inventory.Widget_Inventory_C" self))
  (UserInterface|Viewport|AddtoPlayerScreen _returnvalue)
  (bind _returnvalue_2 (UserInterface|CreateWidget "/Game/Blueprints/Widgets/Widget_Dialogue.Widget_Dialogue_C" self))
  (UserInterface|Viewport|AddtoPlayerScreen _returnvalue_2)
  (bind _asbp_battle_scene_game_mode (Utilities|Casting|CastToBP_BattleSceneGameMode (Game|GetGameMode)))
  (EventDispatchers|AssignOnHandleTurn _asbp_battle_scene_game_mode (EventDispatchers|CreateEvent :!event HandleTurn)))

(fn ConstructionScript)

(fn HandleTurn
  (params (CurrentTurn :type RPG%20Paper%20Character%20Object%20Reference))
  (if (not (== CurrentTurn (Pawn|GetControlledPawn)))
    (Utilities|IsValid (Pawn|GetController CurrentTurn)
      (:Is%20Not%20Valid
        (Pawn|Possess CurrentTurn)
        (bind _returnvalue (UserInterface|CreateWidget "/Game/Blueprints/Widgets/Widget_BattleUI.Widget_BattleUI_C" self))
        (UserInterface|Viewport|AddtoPlayerScreen _returnvalue)))))