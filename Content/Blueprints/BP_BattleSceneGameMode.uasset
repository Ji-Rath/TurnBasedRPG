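; Game mode for a turn-based RPG battle that runs the turn order and decides win or loss.
; On BeginPlay it spawns both Game Instance teams at free, team-matched spawn points, shuffles them into one turn order and broadcasts the first turn.
; EndTurn destroys characters whose health attribute is depleted, then broadcasts the next turn, wrapping around.
; Destroy callbacks prune the lists; an empty team triggers win (delayed) or loss, both opening TestMap.
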(event Custom|HandleWin
  (Utilities|FlowControl|Delay 3.0)
  (Game|OpenLevel(byObjectReference) "/Game/Maps/TestMap.TestMap"))

(event EventBeginPlay
  (CallFunction|SpawnCharacters)
  (Utilities|Array|Shuffle (Variables|Default|GetTurnOrder))
  (Utilities|FlowControl|Delay 0.2)
  (Default|CallOnHandleTurn (Utilities|Array|Get(acopy) (Variables|Default|GetTurnOrder) (Variables|Default|GetTurnIndex))))

(fn ConstructionScript)

(fn SpawnCharacters
  (bind _asbp_rpggame_instance (Utilities|Casting|CastToBP_RPGGameInstance (Game|GetGameInstance)))
  (bind _spawnedactors (CallFunction|SpawnTeam (Variables|/Game/Blueprints/BP_RPGGameInstance.BP_RPGGameInstance_C|GetTeam%201 _asbp_rpggame_instance) 1))
  (Utilities|Array|AppendArray (Variables|Default|GetTurnOrder) _spawnedactors)
  (Variables|Default|SetTeam1Size _spawnedactors)
  (bind _spawnedactors_2 (CallFunction|SpawnTeam (Variables|/Game/Blueprints/BP_RPGGameInstance.BP_RPGGameInstance_C|GetTeam%202 _asbp_rpggame_instance) 2))
  (Utilities|Array|AppendArray (Variables|Default|GetTurnOrder) _spawnedactors_2)
  (Variables|Default|SetTeam2Size _spawnedactors_2))

(fn EndTurn
  (CallFunction|CheckCharactersHP)
  (bind _result (Math|Integer|IncrementInt (Variables|Default|GetTurnIndex))
    (:%20%20
      (if (>= _result (Utilities|Array|Length (Variables|Default|GetTurnOrder)))
        (Variables|Default|SetTurnIndex 0))
      (Default|CallOnHandleTurn (Utilities|Array|Get(acopy) (Variables|Default|GetTurnOrder) (Variables|Default|GetTurnIndex))))))

(fn OnCharacterDestroyed
  (params (DestroyedActor :type Actor%20Object%20Reference))
  (bind _team1size (Variables|Default|GetTeam1Size))
  (bind _team2size (Variables|Default|GetTeam2Size))
  (bind _asrpgpaper_character (Utilities|Casting|CastToRPGPaperCharacter DestroyedActor))
  (Utilities|Array|RemoveItem (Variables|Default|GetTurnOrder) _asrpgpaper_character)
  (if (== (Utilities|Array|FindItem (Variables|Default|GetTeam2Size) _asrpgpaper_character) -1)
    (Utilities|Array|RemoveItem _team1size _asrpgpaper_character)
    (if (<= (Utilities|Array|Length _team1size) 0)
      (CallFunction|HandleLose))
    (else
      (Utilities|Array|RemoveItem _team2size _asrpgpaper_character)
      (if (<= (Utilities|Array|Length _team2size) 0)
        (CallFunction|HandleWin)))))

(fn HandleLose
  (Game|OpenLevel(byObjectReference) "/Game/Maps/TestMap.TestMap"))

(fn CheckCharactersHP
  (for _array_element (Variables|Default|GetTurnOrder)
    (if (.bSuccessfullyFoundAttribute (Ability|Attribute|GetFloatAttribute _array_element "(AttributeName=\"Health\",Attribute=/Script/CoolRPG.RPGAttributeSet:Health,AttributeOwner=None)"))
      (if (<= (.ReturnValue (Ability|Attribute|GetFloatAttribute _array_element "(AttributeName=\"Health\",Attribute=/Script/CoolRPG.RPGAttributeSet:Health,AttributeOwner=None)")) 0.0)
        (Actor|DestroyActor _array_element)))))

(fn SpawnTeam
  (params (Array :type Array%20of%20RPG%20Paper%20Character%20Class%20References) (TeamID :type Integer))
  (for _array_element Array
    (bind _outactors (Actor|GetAllActorsOfClass "/Game/Blueprints/BP_SpawnPoint.BP_SpawnPoint_C"))
    (bind _array_element_2 (Utilities|Array|ForEachLoopwithBreak _outactors :!label _label)
      (:LoopBody
        (if (and (not (Variables|/Game/Blueprints/BP_SpawnPoint.BP_SpawnPoint_C|GetbIsTaken _array_element_2)) (== (Variables|/Game/Blueprints/BP_SpawnPoint.BP_SpawnPoint_C|GetTeamID _array_element_2) TeamID))
          (bind _returnvalue (Game|SpawnActorfromClass _array_element (Transformation|GetActorTransform _array_element_2) "AdjustIfPossibleButAlwaysSpawn" 0 0))
          (Game|BindEventtoOnDestroyed _returnvalue (EventDispatchers|CreateEvent :!event OnCharacterDestroyed))
          (Utilities|Array|Add (LocalVariables|GetSpawnedTeam) _returnvalue)
          (Variables|/Game/Blueprints/BP_SpawnPoint.BP_SpawnPoint_C|SetbIsTaken _array_element_2 true)
          (goto _label Break)))))
  (return (LocalVariables|GetSpawnedTeam)))