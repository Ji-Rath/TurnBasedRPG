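; Generic overworld enemy that starts an RPG battle when the player touches it.
; A Box overlap by BP_Player's capsule, gated on BP_GameMode being active, fires the Interactable component's interaction.
; The interaction handler copies the character's save info into BP_RPGGameInstance.PlayerAttributes.
; It then calls StartBattle with the character's class against this enemy's EnemyTeam, also passing itself as the enemy object.
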(event OnExecuteInteraction(Interactable)
  (params (Interactor :type Actor%20Object%20Reference))
  (bind _asrpgpaper_character (Utilities|Casting|CastToRPGPaperCharacter Interactor))
  (bind _asbp_rpggame_instance (Utilities|Casting|CastToBP_RPGGameInstance (Game|GetGameInstance)))
  (bind _returnvalue (Class|RPGPaperCharacter|GetSaveInfo _asrpgpaper_character))
  (Variables|/Game/Blueprints/BP_RPGGameInstance.BP_RPGGameInstance_C|SetPlayerAttributes _asbp_rpggame_instance _returnvalue)
  (Default|StartBattle _asbp_rpggame_instance (Utilities|Array|MakeArray (Utilities|GetClass _asrpgpaper_character)) (Variables|Default|GetEnemyTeam) (Utilities|Array|MakeArray (Utilities|ResolveSoftReference self))))

(event OnComponentBeginOverlap(Box)
  (params (OverlappedComponent :type Primitive%20Component%20Object%20Reference) (OtherActor :type Actor%20Object%20Reference) (OtherComp :type Primitive%20Component%20Object%20Reference) (OtherBodyIndex :type Integer) (bFromSweep :type Boolean) (SweepResult :type Hit%20Result%20Structure%20%28by%20ref%29))
  (Utilities|Casting|CastToCapsuleComponent OtherComp)
  (Utilities|Casting|CastToBP_GameMode (Game|GetGameMode))
  (Utilities|Casting|CastToBP_Player OtherActor)
  (Default|CallOnInteract (Variables|Default|GetInteractable) OtherActor))

(fn ConstructionScript)