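; Gameplay ability for the pig enemy's special charge attack in turn-based battles, triggered by an Attack.Special1 gameplay event.
; Chained root motion tasks with delays hop it away from the target, charge it in, apply GE_PlayerAttack, bounce back, then return to its saved position.
; Ending the ability tells BP_BattleSceneGameMode to end the turn.
; A capsule-trace helper, GetPosNearTarget, is defined but unused in the event graph.
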(event Ability|EventActivateAbility
  (bind _payload (Ability|Tasks|WaitGameplayEvent "(TagName=\"Attack.Special1\")" 0)
    (:EventReceived
      (Variables|Default|SetIdlePosition (Transformation|GetActorLocation (.Instigator (Utilities|Struct|BreakGameplayEventData _payload))))
      (|ApplyRootMotionJumpForce "None" (Math|Rotator|FindLookatRotation (Transformation|GetActorLocation (.Target (Utilities|Struct|BreakGameplayEventData _payload))) (Transformation|GetActorLocation (.Instigator (Utilities|Struct|BreakGameplayEventData _payload)))) 1e+02 5e+01 0.75 0.0 true "MaintainLastRootMotionVelocity" "0, 0, 0" 0.0 ; Prepare charge attack
        (:OnFinish
          (Utilities|FlowControl|Delay 1.0)
          (Ability|Tasks|ApplyRootMotionMoveToActorForce "None" (.Target (Utilities|Struct|BreakGameplayEventData _payload)) "50.000000,0.000000,0.000000" "AlignFromTargetToSource" 0.5 "/Game/Blueprints/Curve_PigCharge.Curve_PigCharge" 0 false "MOVE_None" false 0 0 "MaintainLastRootMotionVelocity" ; Charge towards player
            (:OnFinished
              (GameplayEffects|ApplyGameplayEffectToTarget (.TargetData (Utilities|Struct|BreakGameplayEventData _payload)) "/Game/Blueprints/GAS/GE_PlayerAttack.GE_PlayerAttack_C" 1 1)
              (|ApplyRootMotionJumpForce "None" (Math|Rotator|FindLookatRotation (Transformation|GetActorLocation (.Target (Utilities|Struct|BreakGameplayEventData _payload))) (Transformation|GetActorLocation (.Instigator (Utilities|Struct|BreakGameplayEventData _payload)))) 1e+02 75.0 0.5 0.0 true "MaintainLastRootMotionVelocity" "0, 0, 0" 0.0 ; Bounce back from player
                (:OnFinish
                  (Utilities|FlowControl|Delay 1.0)
                  (Ability|Tasks|ApplyRootMotionMoveToForce "None" (Variables|Default|GetIdlePosition) 0.5 false "MOVE_None" false 0 "MaintainLastRootMotionVelocity" ; Return to idle location
                    (:OnTimedOutAndDestinationReached
                      (Utilities|FlowControl|Delay 0.5)
                      (Ability|EndAbility))))))))))))

(event Ability|EventOnEndAbility
  (params (bWasCancelled :type Boolean))
  (bind _asbp_battle_scene_game_mode (Utilities|Casting|CastToBP_BattleSceneGameMode (Game|GetGameMode)))
  (Default|EndTurn _asbp_battle_scene_game_mode))

(fn GetPosNearTarget
  (params (Instigator :type Actor%20Object%20Reference) (Target :type Actor%20Object%20Reference))
  (bind (_outhit _returnvalue) (Class|KismetSystemLibrary|CapsuleTraceSinglebyProfile (Transformation|GetActorLocation Instigator) (Transformation|GetActorLocation Target) 4e+01 4e+01 "Pawn" false 0 "None" true))
  (return (select _returnvalue (.Location (Collision|BreakHitResult _outhit)) (.TraceEnd (Collision|BreakHitResult _outhit)))))