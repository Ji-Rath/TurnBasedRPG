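; Player character with flipbook sprite animation, movement input and an interact action forwarded to its interact component.
; Movement axes use the camera's rotation with yaw zeroed.
; On each movement update, velocity against camera axes picks a four-way facing, horizontal first and retaining the last, to choose walk or idle flipbooks.
; It also acts as dialogue participant "Gravy", with stubbed condition, value and event handlers.
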(event EventBeginPlay
  (Character|BindEventtoOnCharacterMovementUpdated (EventDispatchers|CreateEvent :!event BPPlayerAutoGenFunc)))

(event Input|ActionEvents|InputActionInteract
  (params (Key :type Key%20Structure :default "None"))
  (:Pressed
    (Class|PlayerInteractComponent|Interact (Variables|Default|GetBP_PlayerInteractComponent))))

(event Input|AxisEvents|InputAxisMoveForward
  (params (AxisValue :type Float%20%28single-precision%29))
  (bind _camera (Variables|Default|GetCamera))
  (bind _returnvalue (Transformation|GetWorldRotation _camera))
  (Pawn|Input|AddMovementInput (Math|Vector|GetForwardVector (Math|Rotator|MakeRotator (.roll _returnvalue) (.pitch _returnvalue) 0.0)) AxisValue false))

(event Input|AxisEvents|InputAxisMoveRight
  (params (AxisValue :type Float%20%28single-precision%29))
  (bind _camera (Variables|Default|GetCamera))
  (bind _returnvalue (Transformation|GetWorldRotation _camera))
  (Pawn|Input|AddMovementInput (Math|Vector|GetRightVector (Math|Rotator|MakeRotator (.roll _returnvalue) (.pitch _returnvalue) 0.0)) AxisValue false))

(fn ConstructionScript)

(fn BPPlayerAutoGenFunc
  (params (DeltaSeconds :type Float%20%28single-precision%29) (OldLocation :type Vector) (OldVelocity :type Vector))
  (bind _camera (Variables|Default|GetCamera))
  (bind _spritesheet (Variables|Default|GetSpriteSheet))
  (LocalVariables|SetRightSpeed (.y (* OldVelocity (Math|Vector|GetRightVector _camera))))
  (LocalVariables|SetUpSpeed (.x (* OldVelocity (Math|Vector|GetUpVector _camera))))
  (Variables|Default|SetDirection (select (> (LocalVariables|GetRightSpeed) 1.0) "NewEnumerator3" (select (< (LocalVariables|GetRightSpeed) -1.0) "NewEnumerator2" (select (> (LocalVariables|GetUpSpeed) 1.0) "NewEnumerator0" (select (< (LocalVariables|GetUpSpeed) -1.0) "NewEnumerator1" (Variables|Default|GetDirection))))))
  (Sprite|SetFlipbook (Variables|Default|GetSprite) (select (> (Math|Vector|VectorLength OldVelocity) 0.0) (Utilities|Select :Index (Variables|Default|GetDirection) :NewEnumerator0 (.walkup _spritesheet) :NewEnumerator1 (.walkdown _spritesheet) :NewEnumerator2 (.walkleft _spritesheet) :NewEnumerator3 (.walkright _spritesheet)) (Utilities|Select :Index (Variables|Default|GetDirection) :NewEnumerator0 (.idleup _spritesheet) :NewEnumerator1 (.idledown _spritesheet) :NewEnumerator2 (.idleleft _spritesheet) :NewEnumerator3 (.idleright _spritesheet)))))

(fn CheckCondition
  (params (Context :type Dlg%20Context%20Object%20Reference) (ConditionName :type Name :default "None"))
  (return false))

(fn GetBoolValue
  (params (ValueName :type Name :default "None"))
  (return false))

(fn GetFloatValue
  (params (ValueName :type Name :default "None"))
  (return 0.0))

(fn GetIntValue
  (params (ValueName :type Name :default "None"))
  (return 0))

(fn GetNameValue
  (params (ValueName :type Name :default "None"))
  (return "None"))

(fn GetParticipantDisplayName
  (params (ActiveSpeaker :type Name :default "None"))
  (return "Gravy"))

(fn GetParticipantGender
  (return "Masculine"))

(fn GetParticipantIcon
  (params (ActiveSpeaker :type Name :default "None") (ActiveSpeakerState :type Name :default "None"))
  (return 0))

(fn GetParticipantName
  (return "Gravy"))

(fn ModifyBoolValue
  (params (ValueName :type Name :default "None") (bNewValue :type Boolean))
  (return false))

(fn ModifyFloatValue
  (params (ValueName :type Name :default "None") (bDelta :type Boolean) (Value :type Float%20%28single-precision%29))
  (return false))

(fn ModifyIntValue
  (params (ValueName :type Name :default "None") (bDelta :type Boolean) (Value :type Integer))
  (return false))

(fn ModifyNameValue
  (params (ValueName :type Name :default "None") (NameValue :type Name :default "None"))
  (return false))

(fn OnDialogueEvent
  (params (Context :type Dlg%20Context%20Object%20Reference) (EventName :type Name :default "None"))
  (return false))