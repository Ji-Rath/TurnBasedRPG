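; BP_Player is the player character: it handles movement and interaction input and acts as the dialogue participant "Gravy".
; One tick after BeginPlay, it passes the RPG game instance's PlayerAttributes to LoadSaveInfo.
; Move axes follow vectors built from camera roll and pitch with yaw zeroed, and Interact calls the player interact component.
; Apart from name and gender, the dialogue interface functions are stubs returning default values.
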(event EventBeginPlay
  (|CallParentFunction)
  (Utilities|FlowControl|Delay 0.0) ; Needs to be delayed till next tick to function properly
  (bind _asbp_rpggame_instance (Utilities|Casting|CastToBP_RPGGameInstance (Game|GetGameInstance)))
  (Class|RPGPaperCharacter|LoadSaveInfo (Variables|/Game/Blueprints/BP_RPGGameInstance.BP_RPGGameInstance_C|GetPlayerAttributes _asbp_rpggame_instance)))

(event Input|ActionEvents|InputActionInteract
  (params (Key :type Key%20Structure :default "None"))
  (:Pressed
    (Class|InteractorComponent|Interact (Variables|Default|GetBP_PlayerInteractComponent))))

(event Input|AxisEvents|InputAxisMoveForward
  (params (AxisValue :type Float%20%28single-precision%29))
  (bind _camera (Variables|Default|GetCamera))
  (bind _returnvalue (Transformation|GetWorldRotation _camera))
  (Pawn|Input|AddMovementInput (Math|Vector|GetForwardVector (Math|Rotator|MakeRotator (.roll _returnvalue) (.pitch _returnvalue) 0.0)) AxisValue false))

(event Input|AxisEvents|InputAxisMoveRight
  (params (AxisValue :type Float%20%28single-precision%29))
  (bind _camera (Variables|Default|GetCamera))
  (bind _returnvalue (Transformation|GetWorldRotation _camera))
  (Pawn|Input|AddMovementInput (Math|Vector|GetRightVector (Math|Rotator|MakeRotator (.roll _returnvalue) (.pitch _returnvalue) 0.0)) AxisValue false))

(fn ConstructionScript)

(fn OnDialogueEvent
  (params (Context :type Dlg%20Context%20Object%20Reference) (EventName :type Name :default "None"))
  (return false))

(fn ModifyNameValue
  (params (ValueName :type Name :default "None") (NameValue :type Name :default "None"))
  (return false))

(fn ModifyIntValue
  (params (ValueName :type Name :default "None") (bDelta :type Boolean) (Value :type Integer))
  (return false))

(fn ModifyFloatValue
  (params (ValueName :type Name :default "None") (bDelta :type Boolean) (Value :type Float%20%28single-precision%29))
  (return false))

(fn ModifyBoolValue
  (params (ValueName :type Name :default "None") (bNewValue :type Boolean))
  (return false))

(fn GetParticipantName
  (return "Gravy"))

(fn GetParticipantIcon
  (params (ActiveSpeaker :type Name :default "None") (ActiveSpeakerState :type Name :default "None"))
  (return 0))

(fn GetParticipantGender
  (return "Masculine"))

(fn GetParticipantDisplayName
  (params (ActiveSpeaker :type Name :default "None"))
  (return "Gravy"))

(fn GetNameValue
  (params (ValueName :type Name :default "None"))
  (return "None"))

(fn GetIntValue
  (params (ValueName :type Name :default "None"))
  (return 0))

(fn GetFloatValue
  (params (ValueName :type Name :default "None"))
  (return 0.0))

(fn GetBoolValue
  (params (ValueName :type Name :default "None"))
  (return false))

(fn CheckCondition
  (params (Context :type Dlg%20Context%20Object%20Reference) (ConditionName :type Name :default "None"))
  (return false))