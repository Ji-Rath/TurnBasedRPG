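; BP_Slime is a slime enemy that starts a battle when interacted with and takes part in turn-based combat.
; Interaction from an RPGPaperCharacter calls StartBattle on the game instance, passing that character's class and its own class as opposing teams.
; On BeginPlay it binds to the battle game mode's OnHandleTurn, and on its own turn it immediately ends the turn and prints a message.
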(event OnExecuteInteraction(Interactable)
  (params (Interactor :type Actor%20Object%20Reference))
  (bind _asrpgpaper_character (Utilities|Casting|CastToRPGPaperCharacter Interactor))
  (bind _asbp_rpggame_instance (Utilities|Casting|CastToBP_RPGGameInstance (Game|GetGameInstance)))
  (Default|StartBattle _asbp_rpggame_instance (Utilities|Array|MakeArray (Utilities|GetClass _asrpgpaper_character)) (Utilities|Array|MakeArray (Utilities|GetClass self))))

(event Custom|OnHandleTurn_Event_0
  (params (CurrentTurn :type RPG%20Paper%20Character%20Object%20Reference))
  (if (== CurrentTurn self)
    (bind _asbp_battle_scene_game_mode (Utilities|Casting|CastToBP_BattleSceneGameMode (Game|GetGameMode)))
    (Default|EndTurn _asbp_battle_scene_game_mode)
    (Development|PrintString "Slimes turn has ended!" true true "(R=0.000000,G=0.660000,B=1.000000,A=1.000000)" 5.0)))

(event EventBeginPlay
  (bind _asbp_battle_scene_game_mode (Utilities|Casting|CastToBP_BattleSceneGameMode (Game|GetGameMode)))
  (EventDispatchers|AssignOnHandleTurn _asbp_battle_scene_game_mode (delegate Custom|OnHandleTurn_Event_0)))

(fn ConstructionScript)