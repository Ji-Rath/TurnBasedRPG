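; GA_PiggyPound is a gameplay ability for a turn-based battle attack that jumps the attacker at a target and back.
; On an Attack gameplay event it stores the instigator's position, then uses a root motion jump force aimed at the target.
; After landing it applies GE_PlayerAttack to the event's target data, then moves back to the stored position with root motion.
; Ending the ability tells the battle scene game mode to end the turn.
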(event Ability|EventActivateAbility
  (Development|PrintString "PIGGY POUND!!")
  (bind _payload (Ability|Tasks|WaitGameplayEvent "(TagName=\"Attack\")" 0)
    (:EventReceived
      (Variables|Default|SetIdlePosition (Transformation|GetActorLocation (.Instigator (Utilities|Struct|BreakGameplayEventData _payload))))
      (|ApplyRootMotionJumpForce "None" (Math|Rotator|FindLookatRotation (Transformation|GetActorLocation (.Instigator (Utilities|Struct|BreakGameplayEventData _payload))) (Transformation|GetActorLocation (.Target (Utilities|Struct|BreakGameplayEventData _payload)))) 6e+02 1e+02 1.0 0.0 false "MaintainLastRootMotionVelocity" "0, 0, 0" 0.0
        (:OnFinish
          (Utilities|FlowControl|Delay 0.5)
          (GameplayEffects|ApplyGameplayEffectToTarget (.TargetData (Utilities|Struct|BreakGameplayEventData _payload)) "/Game/Blueprints/GAS/GE_PlayerAttack.GE_PlayerAttack_C" 1 1)
          (Utilities|FlowControl|Delay 0.5)
          (Ability|Tasks|ApplyRootMotionMoveToForce "None" (Variables|Default|GetIdlePosition) 0.5 false "MOVE_None" false 0 "MaintainLastRootMotionVelocity"
            (:OnTimedOutAndDestinationReached
              (Utilities|FlowControl|Delay 0.5)
              (Ability|EndAbility))))))))

(event Ability|EventOnEndAbility
  (params (bWasCancelled :type Boolean))
  (bind _asbp_battle_scene_game_mode (Utilities|Casting|CastToBP_BattleSceneGameMode (Game|GetGameMode)))
  (Default|EndTurn _asbp_battle_scene_game_mode))