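; GA_Attack is a Gameplay Ability that performs an attack in a turn-based battle.
; On activation it waits for an Attack gameplay event, then moves the instigator to the target with a swept teleport-free move and applies GE_PlayerAttack to the event's target data.
; After short delays it returns the instigator to its original position and ends.
; On end, it tells BP_BattleSceneGameMode to end the turn.
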(event Ability|EventActivateAbility
  (bind _payload (Ability|Tasks|WaitGameplayEvent "(TagName=\"Attack\")" 0)
    (:EventReceived
      (bind _output_get (Variables|Default|SetIdlePosition (Transformation|GetActorLocation (.Instigator (Utilities|Struct|BreakGameplayEventData _payload)))))
      (Transformation|SetActorLocation (.Instigator (Utilities|Struct|BreakGameplayEventData _payload)) (Transformation|GetActorLocation (.Target (Utilities|Struct|BreakGameplayEventData _payload))) true false)
      (GameplayEffects|ApplyGameplayEffectToTarget (.TargetData (Utilities|Struct|BreakGameplayEventData _payload)) "/Game/Blueprints/GAS/GE_PlayerAttack.GE_PlayerAttack_C" 1 1)
      (Utilities|FlowControl|Delay 1.0)
      (Transformation|SetActorLocation (.Instigator (Utilities|Struct|BreakGameplayEventData _payload)) _output_get true false)
      (Utilities|FlowControl|Delay 1.0)
      (Ability|EndAbility))))

(event Ability|EventOnEndAbility
  (params (bWasCancelled :type Boolean))
  (bind _asbp_battle_scene_game_mode (Utilities|Casting|CastToBP_BattleSceneGameMode (Game|GetGameMode)))
  (Default|EndTurn _asbp_battle_scene_game_mode))