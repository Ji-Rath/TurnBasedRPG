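; Gameplay ability for using an item in a battle, ending the turn afterward.
; On activation it waits for a UseItem gameplay event that carries the target data and the battle UI widget as its optional object.
; It applies the effect stored in that widget's item info to the targets, then ends after a short delay.
; Ending the ability calls EndTurn on the battle scene game mode.
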(event Ability|EventActivateAbility
  (bind _payload (Ability|Tasks|WaitGameplayEvent "(TagName=\"UseItem\")" 0)
    (:EventReceived
      (bind _aswidget_battle_ui (Utilities|Casting|CastToWidget_BattleUI (.OptionalObject (Utilities|Struct|BreakGameplayEventData _payload))))
      (GameplayEffects|ApplyGameplayEffectToTarget (.TargetData (Utilities|Struct|BreakGameplayEventData _payload)) (.effectonuse (Variables|/Game/Blueprints/Widgets/Widget_BattleUI.Widget_BattleUI_C|GetItem%20Info _aswidget_battle_ui)) 1 1)
      (Utilities|FlowControl|Delay 1.0)
      (Ability|EndAbility))))

(event Ability|EventOnEndAbility
  (params (bWasCancelled :type Boolean))
  (bind _asbp_battle_scene_game_mode (Utilities|Casting|CastToBP_BattleSceneGameMode (Game|GetGameMode)))
  (Default|EndTurn _asbp_battle_scene_game_mode))